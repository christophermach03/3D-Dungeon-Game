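; Damage system component that tracks health, death and the blocking, invincible and interruptable states for its owner.
; TakeDamage uses the DetermineIfDamaged macro to route each hit to blocked, ignored or applied, then calls the OnBlocked, OnDeath or OnDamageResponse dispatchers.
; Damage responses fire only when the hit forces an interrupt or the owner is interruptable.
; Heal, while alive, zeroes Health and returns a clamped sum.
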(fn `Heal`
  (params (Amount :type "Float (double-precision)"))
  (returns (NewHealth :type "Float (double-precision)"))
  (if (not (`self.IsDead`))
    (set `self.Health` 0.0)
    (return (`KismetMathLibrary.FClamp` (+ Amount (`self.Health`)) 0.0 (`self.MaxHealth`)))))

(fn `TakeDamage`
  (params (DamageInfo :type "/Game/_CombatSystem/s_DamageInfo Structure"))
  (returns (WasDamaged :type Boolean))
  (bind (_amount _damagetype _damageresponse _canbeblocked _forceinterrupt) (break `/Game/_CombatSystem/s_DamageInfo` DamageInfo))
  (`self.DetermineIfDamaged` _canbeblocked
    (:`BlockDamage`
      (`KismetSystemLibrary.PrintString` "Blocked Damage!!!")
      (`self.OnBlocked`)
      (return false))
    (:`NoDamage`
      (return false))
    (:`DoDamage`
      (bind _output_get (set `self.Health` (- (`self.Health`) _amount)))
      (if (<= _output_get 0.0)
        (set `self.IsDead` true)
        (`self.OnDeath`)
        (return true)
        (elif (or _forceinterrupt (`self.IsInterruptable`))
          (`self.OnDamageResponse` _damageresponse)
          (return true))))))